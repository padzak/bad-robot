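; BP_SmallSpehere is an actor that moves continuously along its forward vector, changing how it turns when it overlaps another actor.
; Tick offsets it by Speed scaled by delta time without sweeping, then adds DeltaRotation, which is not scaled by delta time.
; Each begin overlap replaces DeltaRotation with a random rotator scaled by RotationScaleFactor, so the heading keeps curving in a new direction.
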(event `self.ReceiveActorBeginOverlap`
  (params (OtherActor :type "Actor Object Reference"))
  (set `self.DeltaRotation` (* (`KismetMathLibrary.RandomRotator` false) (`self.RotationScaleFactor`))))

(event `self.ReceiveTick`
  (params (DeltaSeconds :type "Float (single-precision)"))
  (`self.K2_AddActorWorldOffset` (* (* DeltaSeconds (`self.Speed`)) (`self.GetActorForwardVector`)))
  (`self.K2_AddActorWorldRotation` (`self.DeltaRotation`)))

(fn `UserConstructionScript`)