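; BP_SphereSpawner is an actor that repeatedly spawns BP_SmallSpehere actors at random positions within a radius around itself.
; BeginPlay starts a looping timer at SpawnTime intervals that fires SpawnSmallSphere.
; Each spawn location comes from GetRandomPointInSphereRadius, which offsets the actor's location along a random rotator's forward vector by a random distance up to SpawnRadius.
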(event `self.ReceiveBeginPlay`
  (`KismetSystemLibrary.K2_SetTimerDelegate` (delegate `SpawnSmallSphere`) (`self.SpawnTime`) true))

(event `SpawnSmallSphere`
  (`|SpawnActorFromClass` "/Game/Blueprints/SmallSphere/BP_SmallSpehere.BP_SmallSpehere_C" (`KismetMathLibrary.MakeTransform` (`self.GetRandomPointInSphereRadius`)) "Undefined" "MultiplyWithRoot" null null))

(event `self.ReceiveTick`
  (params (DeltaSeconds :type "Float (single-precision)")))

(fn `GetRandomPointInSphereRadius`
  (returns (RandomPoint :type "Vector Structure"))
  (return (+ (`self.K2_GetActorLocation`) (* (`KismetMathLibrary.GetForwardVector` (`KismetMathLibrary.RandomRotator` false)) (`KismetMathLibrary.RandomFloatInRange` 0.0 (`self.SpawnRadius`))))))

(fn `UserConstructionScript`)