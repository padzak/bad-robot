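; BP_Ball is a labeled ball Blueprint that can optionally start moving after a delay.
; On BeginPlay it passes its Label to the WBP_BallWidget in its Widget component, stopping if that cast fails.
; When IsMovingBall is set, it waits for the configured Delay, then calls StartMoving, which only raises the ShouldMove flag.
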(event `self.ReceiveBeginPlay`
  (bind _aswbp_ball_widget (cast `/Game/Blueprints/Widget/WBP_BallWidget` (`WidgetComponent.GetWidget` (`self.Widget`))))
  (set `/Game/Blueprints/Widget/WBP_BallWidget.Label` (`self.Label`) _aswbp_ball_widget)
  (if (`self.IsMovingBall`)
    (`KismetSystemLibrary.Delay` (`self.Delay`))
    (`self.StartMoving`)))

(fn `StartMoving`
  (set `self.ShouldMove` true))

(fn `UserConstructionScript`)