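; Ball actor Blueprint, one of the movement-method variants, that explodes and destroys itself on a hit.
; On BeginPlay it runs the parent logic, then binds to the BallMesh component hit event.
; A hit spawns a fire explosion effect and impact sound at the actor's location before destroying it.
; The AddActorWorldOffset tick movement in its name is not implemented in this graph.
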(event `self.ReceiveBeginPlay`
  (`parent.ReceiveBeginPlay`)
  (add `PrimitiveComponent.OnComponentHit` (`self.BallMesh`) (delegate `OnComponentHit_Event`)))

(event `OnComponentHit_Event`
  (params (HitComponent :type "PrimitiveComponent Object Reference") (OtherActor :type "Actor Object Reference") (OtherComp :type "PrimitiveComponent Object Reference") (NormalImpulse :type "Vector Structure") (Hit :type "HitResult Structure (by ref)"))
  (`NiagaraFunctionLibrary.SpawnSystemAtLocation` "/Game/Global/Effects/Projectiles/FireExplosion/NS_FireExplosion.NS_FireExplosion" (`self.K2_GetActorLocation`))
  (`GameplayStatics.SpawnSoundAtLocation` "/Game/Global/Sounds/Explode/sfx_FireBolt_Impact.sfx_FireBolt_Impact" (`self.K2_GetActorLocation`) (struct) 1.0 1.0 0.0 null null)
  (`self.K2_DestroyActor`))

(fn `UserConstructionScript`
  (`parent.UserConstructionScript`))