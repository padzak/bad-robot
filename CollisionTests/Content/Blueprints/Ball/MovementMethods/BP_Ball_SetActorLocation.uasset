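; Ball actor that demonstrates movement through SetActorLocation, moving along its forward vector.
; BeginPlay caches the starting location in NewLocation.
; While ShouldMove is set, each Tick advances that stored location by Speed times world delta seconds and applies it, with optional sweep and no teleport.
; The position accumulates in the variable rather than being re-read from the actor each frame.
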(event `self.ReceiveBeginPlay`
  (`parent.ReceiveBeginPlay`)
  (set `self.NewLocation` (`self.K2_GetActorLocation`)))

(event `self.ReceiveTick`
  (params (DeltaSeconds :type "Float (single-precision)"))
  (`parent.ReceiveTick` DeltaSeconds)
  (if (`self.ShouldMove`)
    (bind _output_get (set `self.NewLocation` (+ (`self.NewLocation`) (* (`self.GetActorForwardVector`) (* (`self.Speed`) (`GameplayStatics.GetWorldDeltaSeconds`))))))
    (`self.K2_SetActorLocation` _output_get (`self.ShouldSweep`))))

(fn `UserConstructionScript`
  (`parent.UserConstructionScript`))